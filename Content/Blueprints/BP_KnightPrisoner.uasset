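; BP_KnightPrisoner is an interactable knight prisoner that awards experience and cheers when interacted with.
; It loops an idle animation from BeginPlay.
; Interact casts the instigator's PlayerState to US_PlayerState, adds EarnedXp, then calls CharacterCheer to loop the cheer animation, intended for all clients.
; CanInteract always returns false, and nothing in this Blueprint changes that.
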(event `self.ReceiveBeginPlay`
  ;[1 1 1] Start the Idle animation
  (`SkeletalMeshComponent.PlayAnimation` (`self.SkeletalMesh`) (`self.MontageIdle`) true))

(event `self.Interact`
  (params (CharacterInstigator :type "US_Character Object Reference"))
  ;[1 1 1] On interaction, grant the experience points and start the interaction animation
  (bind _asus_player_state (cast `US_PlayerState` (`Pawn.PlayerState` CharacterInstigator)))
  (`US_PlayerState.AddXp` _asus_player_state (`self.EarnedXp`))
  (`self.CharacterCheer`))

(event `CharacterCheer`
  ;[1 1 1] Start the Cheer animation on all clients
  (`SkeletalMeshComponent.PlayAnimation` (`self.SkeletalMesh`) (`self.MontageCheer`) true))

(fn `CanInteract`
  (params (CharacterInstigator :type "Character Object Reference"))
  (returns (ReturnValue :type Boolean))
  (return false))

(fn `UserConstructionScript`)