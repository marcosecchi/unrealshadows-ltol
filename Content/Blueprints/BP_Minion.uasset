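; BP_Minion is an AI-driven minion pawn that wanders to random reachable navmesh points within a very large radius.
; A Patrol event issues the AI MoveTo toward a new random point.
; Tick calls Patrol after a delay when max movement speed exceeds PatrolSpeed and no valid TargetCharacter exists; nothing here sets that target.
; An unconnected SimpleMoveToLocation and debug-sphere draw remain in the graph.
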(event `Patrol`
  (`|AIMoveTo` self (`NavigationSystemV1.K2_GetRandomReachablePointInRadius` (`self.K2_GetActorLocation`) 50000.0 null null) null))

(event `self.ReceiveTick`
  (params (DeltaSeconds :type "Float (single-precision)"))
  (if (> (`MovementComponent.GetMaxSpeed` (`self.CharacterMovement`)) (`self.PatrolSpeed`))
    (`KismetSystemLibrary.Delay` 5.0)
    (`self.TargetCharacter`
      (:`then`)
      (:`else`
        (`self.PAtrol`)))))

(fn `UserConstructionScript`)