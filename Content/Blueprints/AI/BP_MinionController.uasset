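; BP_MinionController is an AI controller for minions that starts the BT_Minion behavior tree on possession.
; It seeds the PatrolLocation blackboard key with one hardcoded world position.
; The perception update event is empty; disconnected nodes would flag line of sight and store a sensed US_Character as ThiefCharacter, but they never run.
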(event `self.ReceivePossess`
  (params (PossessedPawn :type "Pawn Object Reference"))
  (`self.RunBehaviorTree` "/Game/Blueprints/AI/BT_Minion.BT_Minion")
  (`BlackboardComponent.SetValueAsVector` (`self.Blackboard`) (`self.PatrolLocation`) (-4439.999996 -8100.000004 96.000007)))

(event `self.AIPerception.OnTargetPerceptionUpdated`
  (params (Actor :type "Actor Object Reference") (Stimulus :type "AIStimulus Structure")))

(fn `UserConstructionScript`)