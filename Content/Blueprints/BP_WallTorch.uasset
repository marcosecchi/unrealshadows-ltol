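; BP_WallTorch is a wall torch Blueprint that makes its light flicker.
; On Tick, a countdown timer triggers a new random intensity for the FlickeringLight component, kept between the MinLightIntensity and MaxLightIntensity variables.
; Each change also resets the timer to a short random interval, so the flicker has an irregular rhythm and jumps between values without interpolation.
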(event `self.ReceiveTick`
  (params (DeltaSeconds :type "Float (single-precision)"))
  (if (<= (`self.Timer`) 0.0)
    (set `self.Timer` (`KismetMathLibrary.RandomFloatInRange` 0.01 0.08))
    (`LightComponent.SetIntensity` (`self.FlickeringLight`) (`KismetMathLibrary.RandomFloatInRange` (`self.MinLightIntensity`) (`self.MaxLightIntensity`)))
    (else
      (set `self.Timer` (- (`self.Timer`) DeltaSeconds)))))

(fn `UserConstructionScript`)